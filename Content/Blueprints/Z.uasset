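; Round-based spawner that creates EvilCubePawn enemies at TargetPoints near the player and tracks the live cubes.
; SpawnAI respects a round quota and live-count cap, picking randomly from up to three spawn points filtered by player distance.
; DeleteItem removes cubes; an empty array starts a new round with a larger quota and notifies EvilCubeHud.
; ChooseSpecificSpawn is uncalled here, and FindClosestSpawn is an empty stub.
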(event `SpawnAI`
  (if (!= (`self.EvilCubesLeft`) 0)
    (if (<= (`KismetArrayLibrary.Array_Length` (`self.EvilCubeArray`)) (`self.MaxEvilCubes`))
      (bind _chosenspawnposition (`self.ChooseRandomSpawn`))
      (bind _returnvalue (`AIBlueprintHelperLibrary.SpawnAIFromClass` "/Game/Blueprints/EvilCubePawn.EvilCubePawn_C" null (`KismetMathLibrary.TransformLocation` _chosenspawnposition) (`KismetMathLibrary.TransformRotation` _chosenspawnposition) true null))
      (bind _asevil_cube_pawn (cast `/Game/Blueprints/EvilCubePawn` _returnvalue))
      (`KismetArrayLibrary.Array_Add` (`self.EvilCubeArray`) _asevil_cube_pawn)
      (`/Engine/EditorBlueprintResources/StandardMacros.DecrementInt` (`self.EvilCubesLeft`)))))

(event `Delete Item`
  (params (EvilCubeToDestroy :type "/Game/Blueprints/EvilCubePawn Object Reference"))
  (bind _rounds (`self.Rounds`))
  (`KismetArrayLibrary.Array_RemoveItem` (`self.EvilCubeArray`) EvilCubeToDestroy)
  (if (== (`KismetArrayLibrary.Array_Length` (`self.EvilCubeArray`)) 0)
    (`/Engine/EditorBlueprintResources/StandardMacros.IncrementInt` _rounds
      (:`  `
        (bind _output_get (set `self.totalCubesPerRound` (+ 25 (`KismetMathLibrary.FTrunc` (* _rounds 5.0)))))
        (set `self.EvilCubesLeft` _output_get)
        (bind _asevil_cube_hud (cast `/Game/EvilCubeHud` (`PlayerController.GetHUD` (`GameplayStatics.GetPlayerController` 0))))
        (`/Game/EvilCubeHud.New Round` _asevil_cube_hud)))))

(fn `ChooseRandomSpawn`
  (returns (ChosenSpawnPosition :type "Transform Structure"))
  (locals (NewLocalVar_0 :type String :default "Chosen Spawn: "))
  (bind _outactors (`GameplayStatics.GetAllActorsOfClass` "/Script/Engine.TargetPoint"))
  (bind _closestspawns (`self.GetArrayOfClosestSpawns` _outactors))
  (bind _returnvalue (`KismetArrayLibrary.Array_Length` _closestspawns))
  (if (== 0 _returnvalue)
    (`KismetSystemLibrary.PrintString` "array empty")
    (else
      (bind _output (`|GetArrayItem` _closestspawns (`KismetMathLibrary.RandomIntegerInRange` 0 (- _returnvalue 1))))
      (`KismetSystemLibrary.PrintString` (`KismetStringLibrary.Concat_StrStr` (`local.NewLocalVar_0`) (`KismetSystemLibrary.GetDisplayName` _output)))
      (return (`self.GetTransform` _output)))))

(fn `ChooseSpecificSpawn`
  (returns (chosenSpawn :type "TargetPoint Object Reference"))
  (locals (bestSpawn :type "TargetPoint Object Reference"))
  (bind _outactors (`GameplayStatics.GetAllActorsOfClass` "/Script/Engine.TargetPoint"))
  (set `self.minSpawnDistance` 10000.0)
  (for _array_element _outactors
    (bind _distance (`self.GetDistanceBetweenTargetAndPlayer` _array_element))
    (if (< _distance (`self.minSpawnDistance`))
      (set `self.minSpawnDistance` 0.0)
      (set `local.bestSpawn` _array_element)))
  (return (`local.bestSpawn`)))

(fn `Find Closest Spawn`
  (params (targetSpawn :type "Array of TargetPoint Object Reference"))
  (locals (bestSpawn :type "TargetPoint Object Reference")))

(fn `GetArrayOfClosestSpawns`
  (params (allSpawns :type "Array of TargetPoint Object Reference"))
  (returns (closestSpawns :type "Array of TargetPoint Object Reference"))
  (locals (bestSpawns :type "Array of TargetPoint Object Reference") (currentSpawn :type "TargetPoint Object Reference"))
  (bind _bestspawns (`local.bestSpawns`))
  (bind _bestspawns_2 (`local.bestSpawns`))
  (for _array_element allSpawns
    (set `local.currentSpawn` _array_element)
    (if (< (`KismetArrayLibrary.Array_Length` (`local.bestSpawns`)) 3)
      (`KismetArrayLibrary.Array_Add` _bestspawns (`local.currentSpawn`) :!label _label)
      (else
        (bind _distance (`self.GetDistanceBetweenTargetAndPlayer` (`local.currentSpawn`)))
        (for _array_element_2 (`local.bestSpawns`)
          (bind _distance_2 (`self.GetDistanceBetweenTargetAndPlayer` _array_element_2))
          (if (> _distance_2 _distance)
            (`KismetArrayLibrary.Array_RemoveItem` _bestspawns _array_element_2)
            (goto _label))))))
  (if (== (`KismetArrayLibrary.Array_Length` _bestspawns_2) 0)
    (`KismetSystemLibrary.PrintString` "no spawns chosen"))
  (return _bestspawns_2))

(fn `GetDistanceBetweenTargetAndPlayer`
  (params (spawnPoint :type "TargetPoint Object Reference"))
  (returns (distance :type "Float (double-precision)"))
  (return (`KismetMathLibrary.Vector_Distance` (`SceneComponent.K2_GetComponentLocation` (`TargetPoint.SpriteComponent` spawnPoint)) (`SceneComponent.K2_GetComponentLocation` (`Character.CapsuleComponent` (`GameplayStatics.GetPlayerCharacter` 0))))))

(fn `UserConstructionScript`)
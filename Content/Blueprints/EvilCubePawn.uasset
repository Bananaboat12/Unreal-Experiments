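; EvilCubePawn is a hazard cube pawn that explodes when its cube component hits something.
; On hit it spawns an explosion effect at the cube's transform, asks the Z game mode to delete it from its items, then destroys the cube component.
; The pawn destroys itself only when the spawned explosion effect ends play, so its lifetime follows the effect.
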(event `self.Cube.OnComponentHit`
  (params (HitComponent :type "PrimitiveComponent Object Reference") (OtherActor :type "Actor Object Reference") (OtherComp :type "PrimitiveComponent Object Reference") (NormalImpulse :type "Vector Structure") (Hit :type "HitResult Structure (by ref)"))
  (bind _cube (`self.Cube`))
  (`|ExecutionSequence`
    (:`then_0`
      (bind _returnvalue (`|SpawnActorFromClass` "/Game/StarterContent/Blueprints/Blueprint_Effect_Explosion.Blueprint_Effect_Explosion_C" (`SceneComponent.K2_GetComponentToWorld` _cube) "Undefined" "OverrideRootScale" null null))
      (set `self.Fire Explosion` _returnvalue)
      (bind _asz (cast `/Game/Blueprints/Z` (`GameplayStatics.GetGameMode`)))
      (`/Game/Blueprints/Z.Delete Item` _asz self))
    (:`then_1`
      (`ActorComponent.K2_DestroyComponent` _cube))))

(event `self.Fire Explosion.OnEndPlay`
  (params (Actor :type "Actor Object Reference") (EndPlayReason :type "EEndPlayReason Enum" :default "Destroyed"))
  (`self.K2_DestroyActor`))

(fn `UserConstructionScript`)